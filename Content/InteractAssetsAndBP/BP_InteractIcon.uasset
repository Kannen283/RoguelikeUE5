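; BP_InteractIcon is an icon actor that turns to face the player's camera.
; BeginPlay starts a looping timer that runs RotateTowardsPlayer in place of Tick, using MainCharacter_BP's camera location as the look-at target.
; Only yaw follows the camera, with pitch and roll fixed.
; The lerp alpha climbs to one and never resets, so the yaw eases in briefly, then snaps to the camera on each update.
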(event `self.ReceiveBeginPlay`
  (`KismetSystemLibrary.K2_SetTimerDelegate` (delegate `RotateTowardsPlayer`) 0.05 true))

(event `RotateTowardsPlayer`
  (bind _lerprotation (`self.LerpRotation`))
  (bind _asmain_character_bp (cast `/Game/MainCharacter/MainCharacter_BP` (`GameplayStatics.GetPlayerCharacter` 0)))
  (set `self.LerpRotation` (`KismetMathLibrary.FClamp` (+ _lerprotation 0.1)))
  (bind (_returnvalue_roll _returnvalue_pitch _returnvalue_yaw) (`KismetMathLibrary.BreakRotator` (`KismetMathLibrary.RLerp` (`self.K2_GetActorRotation`) (`KismetMathLibrary.FindLookAtRotation` (`self.K2_GetActorLocation`) (`SceneComponent.K2_GetComponentLocation` (`/Game/MainCharacter/MainCharacter_BP.Camera` _asmain_character_bp))) _lerprotation)))
  (`self.K2_SetActorRotation` (`KismetMathLibrary.MakeRotator` 0.0 30.0 _returnvalue_yaw)))

(fn `UserConstructionScript`)