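; Player character for a room-based dungeon crawler, handling movement, charge-limited dashing, shooting, health, death, pause and portal interaction.
; FireProjectile spawns single, double or triple shots offset by facing, looping while fire is held.
; Enemy overlaps drain health with temporary immortality, updating the HUD; death returns to the hub level.
; Portals advance MainGameMode's floor, reroll room types and swap presets behind a camera fade; number keys are test hooks.
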(event `self.ReceiveBeginPlay`
  (`|ExecutionSequence`
    (:`then_0`
      ;[1 1 1] Initializing Widgets (For now only HUD)
      (bind _returnvalue (`|CreateWidget` "/Game/MainCharacter/Hud/WD_HUD.WD_HUD_C"))
      (bind _output_get (set `self.WD_HUD_ref` _returnvalue))
      (`UserWidget.AddToViewport` _output_get 0))
    (:`then_1`
      ;[1 1 1] Main Character Mapping
      (bind _asplayer_controller (cast `PlayerController` (`self.GetController`)))
      (bind _returnvalue_2 (pcsubsystem `EnhancedInputLocalPlayerSubsystem` _asplayer_controller))
      (`/Engine/EditorBlueprintResources/StandardMacros.IsValid` _returnvalue_2
        (:`Is Valid`
          (`EnhancedInputSubsystemInterface.AddMappingContext` _returnvalue_2 "/Game/MainCharacter/Input_KeyboardAndMouse/IMC_MainCharacter.IMC_MainCharacter" 0 (struct)))))))

(event `Key|Two`
  (params (Key :type "Key Structure"))
  ;[0.5751 0.05065 1] Increasing HP bars (Test only)
  (:`Pressed`
    (bind _result (`/Engine/EditorBlueprintResources/StandardMacros.IncrementInt` (`self.NumberOfHealthBars`))
      (:`  `
        (set `self.NumberOfHealthBars` (`KismetMathLibrary.Clamp` _result 3 6))
        (`/Game/MainCharacter/Hud/WD_HUD.AddNewHealthBar` (`self.WD_HUD_ref`))
        ;[0.5751 0.05065 1] Increase / decrease health (TEST only)
        (bind _result_2 (`/Engine/EditorBlueprintResources/StandardMacros.IncrementInt` (`self.Health`) :!label _label)
          (:`  `
            (set `self.Health` (`KismetMathLibrary.Clamp` _result_2 0 (`self.NumberOfHealthBars`)))
            (`/Game/MainCharacter/Hud/WD_HUD.Decrease/IncreaseHealthOnHUD` (`self.WD_HUD_ref`) :!label _label_2)))))))

(event `Key|Three`
  (params (Key :type "Key Structure"))
  ;[0.5751 0.05065 1] Increase / decrease health (TEST only)
  (:`Pressed`
    (goto _label)))

(event `EnhancedInput|/Game/MainCharacter/Input_KeyboardAndMouse/IA_MovementWASD`
  (params (ActionValue :type "Vector2D Structure") (ElapsedSeconds :type "Float (double-precision)") (TriggeredSeconds :type "Float (double-precision)") (InputAction :type "InputAction Object Reference" :default "/Game/MainCharacter/Input_KeyboardAndMouse/IA_MovementWASD.IA_MovementWASD"))
  (bind (_returnvalue_roll _returnvalue_pitch _returnvalue_yaw) (`KismetMathLibrary.BreakRotator` (`self.GetControlRotation`)))
  (bind (_returnvalue_roll_2 _returnvalue_pitch_2 _returnvalue_yaw_2) (`KismetMathLibrary.BreakRotator` (`self.GetControlRotation`)))
  ;[1 1 1] Main Character Movement
  (:`Triggered`
    (`self.AddMovementInput` (`KismetMathLibrary.GetRightVector` (`KismetMathLibrary.MakeRotator` _returnvalue_roll_2 0.0 _returnvalue_yaw_2)) ActionValue_X)
    (`self.AddMovementInput` (`KismetMathLibrary.GetForwardVector` (`KismetMathLibrary.MakeRotator` 0.0 0.0 _returnvalue_yaw)) ActionValue_Y)))

(event `Key|Four`
  (params (Key :type "Key Structure"))
  ;[0.5751 0.05065 1] Increase / decrease health (TEST only)
  (:`Pressed`
    (bind _result (`/Engine/EditorBlueprintResources/StandardMacros.DecrementInt` (`self.Health`))
      (:`  `
        (set `self.Health` (`KismetMathLibrary.Clamp` _result 0 (`self.NumberOfHealthBars`)))
        (goto _label_2)))))

(event `Resume`
  ;[0.3369 1 0.2919] Pause
  (set `self.isPauseOpen?` false :!label _label_3)
  (`Widget.RemoveFromParent` (`self.Pause_Ref`))
  (`WidgetBlueprintLibrary.SetInputMode_GameOnly` (`GameplayStatics.GetPlayerController` 0))
  (`GameplayStatics.SetViewportMouseCaptureMode` "CapturePermanently_IncludingInitialMouseDown")
  (`GameplayStatics.SetGamePaused` false)
  (`self.K2_DestroyActor` (stale `EnhancedInput|/Game/MainCharacter/Input_KeyboardAndMouse/IA_Pause` _returnvalue_3)))

(event `EnhancedInput|/Game/MainCharacter/Input_KeyboardAndMouse/IA_MovementDash`
  (params (ActionValue :type Boolean) (ElapsedSeconds :type "Float (double-precision)") (TriggeredSeconds :type "Float (double-precision)") (InputAction :type "InputAction Object Reference" :default "/Game/MainCharacter/Input_KeyboardAndMouse/IA_MovementDash.IA_MovementDash"))
  (bind (_returnvalue_x _returnvalue_y) (`KismetMathLibrary.BreakVector` (`self.GetVelocity`)))
  (bind _charactermovement (`self.CharacterMovement`))
  (bind _returnvalue (`KismetMathLibrary.MakeVector` _returnvalue_x _returnvalue_y))
  (bind _maxwalkspeed (`CharacterMovementComponent.MaxWalkSpeed` (`self.CharacterMovement`)))
  (bind _returnvalue_2 (`KismetMathLibrary.VSize` _returnvalue))
  ;[1 1 1] Dash
  (:`Started`
    (if (and (> (`self.NumberOfDashesHUD`) 0) (not (`self.isDashing?`)) (>= (`KismetMathLibrary.VSize` (`MovementComponent.Velocity` _charactermovement)) 1.0) (not (`NavMovementComponent.IsFalling` _charactermovement)))
      (set `self.isDashing?` true)
      (if (== _returnvalue_2 _maxwalkspeed)
        (`self.LaunchCharacter` (* _returnvalue (`self.DashMultiplier(Distance)`)))
        (else
          (set `self.NewDashMultiplier(NewDistance)` (* (`self.DashMultiplier(Distance)`) (/ _maxwalkspeed _returnvalue_2)))
          (`self.LaunchCharacter` (* _returnvalue (`self.NewDashMultiplier(NewDistance)`)))))
      (`|ExecutionSequence`
        (:`then_0`
          (`KismetSystemLibrary.Delay` 0.15)
          (`MovementComponent.StopMovementImmediately` (`self.CharacterMovement`))
          (`self.DelayBetweenDashes`))
        (:`then_1`
          (`/Engine/EditorBlueprintResources/StandardMacros.DecrementInt` (`self.NumberOfDashesHUD`)
            (:`  `
              (`/Game/MainCharacter/Hud/WD_HUD.ReloadDash_HUD` (`self.WD_HUD_ref`))
              (`self.ReloadDash`))))))))

(event `EnhancedInput|/Game/MainCharacter/Input_KeyboardAndMouse/IA_Pause`
  (params (ActionValue :type Boolean) (ElapsedSeconds :type "Float (double-precision)") (TriggeredSeconds :type "Float (double-precision)") (InputAction :type "InputAction Object Reference" :default "/Game/MainCharacter/Input_KeyboardAndMouse/IA_Pause.IA_Pause"))
  (bind _returnvalue (`GameplayStatics.GetPlayerController` 0))
  ;[0.3369 1 0.2919] Pause
  (:`Started`
    (if (`self.isPauseOpen?`)
      (if (not (`self.inConfirmWidget?`))
        (goto _label_3))
      (else
        (set `self.isPauseOpen?` true)
        (bind _returnvalue_2 (`|CreateWidget` "/Game/MainMenu/Pause_Menu/WD_Pause_Menu.WD_Pause_Menu_C" _returnvalue))
        (bind _output_get (set `self.Pause_Ref` _returnvalue_2))
        (`UserWidget.AddToViewport` _output_get 1)
        (`WidgetBlueprintLibrary.SetInputMode_GameAndUIEx` _returnvalue (`self.Pause_Ref`) "DoNotLock" false)
        (bind _returnvalue_3 (`|SpawnActorFromClass` "/Game/MainMenu/Pause_Menu/OverlayActor.OverlayActor_C" (`KismetMathLibrary.MakeTransform` (500.0 500.0 100.0)) "Undefined" "OverrideRootScale" null null))
        (set `self.OverlayCharacter_Ref` _returnvalue_3)
        (`GameplayStatics.SetGamePaused` true)))))

(event `ReloadDash`
  (bind _numberofdasheshud (`self.NumberOfDashesHUD`))
  ;[1 1 1] Dash
  (`KismetSystemLibrary.Delay` (`self.DashReloadTime`))
  (`/Engine/EditorBlueprintResources/StandardMacros.IncrementInt` _numberofdasheshud
    (:`  `
      (`/Game/MainCharacter/Hud/WD_HUD.ReloadDash_HUD` (`self.WD_HUD_ref`))
      (if (not (== _numberofdasheshud (`self.NumberOfDashes`)))
        (`self.ReloadDash`)))))

(event `DelayBetweenDashes`
  ;[1 1 1] Dash
  (`KismetSystemLibrary.Delay` 0.4)
  (set `self.isDashing?` false))

(event `EnhancedInput|/Game/MainCharacter/Input_KeyboardAndMouse/IA_Interact`
  (params (ActionValue :type Boolean) (ElapsedSeconds :type "Float (double-precision)") (TriggeredSeconds :type "Float (double-precision)") (InputAction :type "InputAction Object Reference" :default "/Game/MainCharacter/Input_KeyboardAndMouse/IA_Interact.IA_Interact"))
  ;[1 1 1] Interact
  (:`Started`
    (if (`self.CharacterInDungeonEntryPortal`)
      (`GameplayStatics.OpenLevelBySoftObjectPtr` "/Game/Dungeon.Dungeon")
      (elif (or (`self.characterInPortal_Right`) (`self.characterInPortal_Left`))
        (`KismetSystemLibrary.PrintString` "Overlap")
        (bind _asmain_game_mode (cast `/Game/MainCharacter/MainGameMode` (`GameplayStatics.GetGameMode`)))
        (bind _floornumber (`/Game/MainCharacter/MainGameMode.FloorNumber` _asmain_game_mode))
        (set `/Game/MainCharacter/MainGameMode.FloorNumber` (+ _floornumber 1) _asmain_game_mode)
        (`KismetSystemLibrary.PrintString` (`KismetStringLibrary.Conv_IntToString` _floornumber))
        (if (<= _floornumber 10)
          (`/Game/MainCharacter/MainGameMode.LP_1/9` _asmain_game_mode)
          (`/Game/MainCharacter/MainGameMode.RandomTypeOfRoom_For_Left` _asmain_game_mode)
          (`/Game/MainCharacter/MainGameMode.RP_1/9` _asmain_game_mode)
          (`/Game/MainCharacter/MainGameMode.RandomTypeOfRoom_For_Right` _asmain_game_mode)
          (`self.EnterPortal`)
          (if (== _floornumber 10)
            (`KismetSystemLibrary.PrintString` "SHOOOOOOOOOOOOOOOP")
            (bind _asmain_game_mode_2 (cast `/Game/MainCharacter/MainGameMode` (`GameplayStatics.GetGameMode`)))
            (set `/Game/MainCharacter/MainGameMode.HardFight` 6.25 _asmain_game_mode_2)
            (set `/Game/MainCharacter/MainGameMode.Survive` 12.5 _asmain_game_mode_2)
            (set `/Game/MainCharacter/MainGameMode.NormalFight` 99.99 _asmain_game_mode_2)
            (set `/Game/MainCharacter/MainGameMode.pickedHard` false _asmain_game_mode_2)
            (set `/Game/MainCharacter/MainGameMode.pickedHard` false _asmain_game_mode_2)
            (set `/Game/MainCharacter/MainGameMode.Shop` 0.0 _asmain_game_mode_2)
            (set `/Game/MainCharacter/MainGameMode.Heal` 0.0 _asmain_game_mode_2)
            (set `/Game/MainCharacter/MainGameMode.pickedShop` false _asmain_game_mode_2)
            (set `/Game/MainCharacter/MainGameMode.pickedHeal` false _asmain_game_mode_2))
          (else
            (`/Game/MainCharacter/MainGameMode.LP_11/19` _asmain_game_mode)
            (`/Game/MainCharacter/MainGameMode.RandomTypeOfRoom_For_Left` _asmain_game_mode)
            (`/Game/MainCharacter/MainGameMode.RP_11/19` _asmain_game_mode)
            (`/Game/MainCharacter/MainGameMode.RandomTypeOfRoom_For_Right` _asmain_game_mode)
            (`self.EnterPortal`)
            (if (== _floornumber 20)
              (`KismetSystemLibrary.PrintString` "HEEEEEEEEEEEEEEEEEEEEEEAL"))
            (if (== _floornumber 21)
              (`KismetSystemLibrary.PrintString` "BOOOOOOOOOOOS"))))))))

(event `FireProjectile`
  (bind (_returnvalue_x _returnvalue_y _returnvalue_z) (`KismetMathLibrary.BreakVector` (`self.K2_GetActorLocation`)))
  (bind (_returnvalue_x_2 _returnvalue_y_2 _returnvalue_z_2) (`KismetMathLibrary.BreakVector` (`self.K2_GetActorLocation`)))
  (bind (_returnvalue_x_3 _returnvalue_y_3 _returnvalue_z_3) (`KismetMathLibrary.BreakVector` (`self.K2_GetActorLocation`)))
  (bind (_returnvalue_x_4 _returnvalue_y_4 _returnvalue_z_4) (`KismetMathLibrary.BreakVector` (`self.K2_GetActorLocation`)))
  (bind (_returnvalue_x_5 _returnvalue_y_5 _returnvalue_z_5) (`KismetMathLibrary.BreakVector` (`self.K2_GetActorLocation`)))
  (bind (_returnvalue_x_6 _returnvalue_y_6 _returnvalue_z_6) (`KismetMathLibrary.BreakVector` (`self.K2_GetActorLocation`)))
  (bind (_returnvalue_x_7 _returnvalue_y_7 _returnvalue_z_7) (`KismetMathLibrary.BreakVector` (`self.K2_GetActorLocation`)))
  (bind (_returnvalue_x_8 _returnvalue_y_8 _returnvalue_z_8) (`KismetMathLibrary.BreakVector` (`self.K2_GetActorLocation`)))
  ;[1 1 1] Fire Projectile
  (if (`self.DoubleShot`)
    (bind _returnvalue (`self.CheckTopBotOrientation`))
    (if _returnvalue
      (`|SpawnActorFromClass` "/Game/MainCharacter/MainCharacterProjectiles/MainCharacterSimpleProjectile.MainCharacterSimpleProjectile_C" (`KismetMathLibrary.MakeTransform` (`KismetMathLibrary.MakeVector` _returnvalue_x_2 (+ _returnvalue_y_2 70.0) _returnvalue_z_2) (`self.K2_GetActorRotation`)) "Undefined" "OverrideRootScale" null (`self.ProjectileSpeed`) null)
      (`|SpawnActorFromClass` "/Game/MainCharacter/MainCharacterProjectiles/MainCharacterSimpleProjectile.MainCharacterSimpleProjectile_C" (`KismetMathLibrary.MakeTransform` (`KismetMathLibrary.MakeVector` _returnvalue_x_3 (+ _returnvalue_y_3 -70.0) _returnvalue_z_3) (`self.K2_GetActorRotation`)) "Undefined" "OverrideRootScale" null (`self.ProjectileSpeed`) null)
      (`KismetSystemLibrary.Delay` (`self.FireRate`) :!label _label_4)
      (if (and (`self.HoldFire`) (not (`self.Reloading`))) :!label _label_5
        (`self.FireProjectile`))
      (else
        (bind _returnvalue_2 (`self.CheckRightLeftOrientation`))
        (if _returnvalue_2
          (`|SpawnActorFromClass` "/Game/MainCharacter/MainCharacterProjectiles/MainCharacterSimpleProjectile.MainCharacterSimpleProjectile_C" (`KismetMathLibrary.MakeTransform` (`KismetMathLibrary.MakeVector` (+ _returnvalue_x_4 70.0) _returnvalue_y_4 _returnvalue_z_4) (`self.K2_GetActorRotation`)) "Undefined" "OverrideRootScale" null (`self.ProjectileSpeed`) null)
          (`|SpawnActorFromClass` "/Game/MainCharacter/MainCharacterProjectiles/MainCharacterSimpleProjectile.MainCharacterSimpleProjectile_C" (`KismetMathLibrary.MakeTransform` (`KismetMathLibrary.MakeVector` (+ _returnvalue_x_5 -70.0) _returnvalue_y_5 _returnvalue_z_5) (`self.K2_GetActorRotation`)) "Undefined" "OverrideRootScale" null (`self.ProjectileSpeed`) null)
          (goto _label_4))))
    (elif (`self.TripleShot`)
      (bind _returnvalue_3 (`self.CheckTopBotOrientation`))
      (if _returnvalue_3
        (`|SpawnActorFromClass` "/Game/MainCharacter/MainCharacterProjectiles/MainCharacterSimpleProjectile.MainCharacterSimpleProjectile_C" (`KismetMathLibrary.MakeTransform` (`KismetMathLibrary.MakeVector` _returnvalue_x_7 (+ _returnvalue_y_7 70.0) _returnvalue_z_7) (`self.K2_GetActorRotation`)) "Undefined" "OverrideRootScale" null (`self.ProjectileSpeed`) null)
        (`|SpawnActorFromClass` "/Game/MainCharacter/MainCharacterProjectiles/MainCharacterSimpleProjectile.MainCharacterSimpleProjectile_C" (`KismetMathLibrary.MakeTransform` (`KismetMathLibrary.MakeVector` _returnvalue_x_8 (+ _returnvalue_y_8 -70.0) _returnvalue_z_8) (`self.K2_GetActorRotation`)) "Undefined" "OverrideRootScale" null (`self.ProjectileSpeed`) null)
        (`|SpawnActorFromClass` "/Game/MainCharacter/MainCharacterProjectiles/MainCharacterSimpleProjectile.MainCharacterSimpleProjectile_C" (`KismetMathLibrary.MakeTransform` (`self.K2_GetActorLocation`) (`self.K2_GetActorRotation`)) "Undefined" "OverrideRootScale" null (`self.ProjectileSpeed`) null)
        (goto _label_4)
        (else
          (bind _returnvalue_4 (`self.CheckRightLeftOrientation`))
          (if _returnvalue_4
            (`|SpawnActorFromClass` "/Game/MainCharacter/MainCharacterProjectiles/MainCharacterSimpleProjectile.MainCharacterSimpleProjectile_C" (`KismetMathLibrary.MakeTransform` (`KismetMathLibrary.MakeVector` (+ _returnvalue_x_6 70.0) _returnvalue_y_6 _returnvalue_z_6) (`self.K2_GetActorRotation`)) "Undefined" "OverrideRootScale" null (`self.ProjectileSpeed`) null)
            (`|SpawnActorFromClass` "/Game/MainCharacter/MainCharacterProjectiles/MainCharacterSimpleProjectile.MainCharacterSimpleProjectile_C" (`KismetMathLibrary.MakeTransform` (`KismetMathLibrary.MakeVector` (+ _returnvalue_x -70.0) _returnvalue_y _returnvalue_z) (`self.K2_GetActorRotation`)) "Undefined" "OverrideRootScale" null (`self.ProjectileSpeed`) null)
            (`|SpawnActorFromClass` "/Game/MainCharacter/MainCharacterProjectiles/MainCharacterSimpleProjectile.MainCharacterSimpleProjectile_C" (`KismetMathLibrary.MakeTransform` (`self.K2_GetActorLocation`) (`self.K2_GetActorRotation`)) "Undefined" "OverrideRootScale" null (`self.ProjectileSpeed`) null)
            (goto _label_4))))
      (else
        (`|SpawnActorFromClass` "/Game/MainCharacter/MainCharacterProjectiles/MainCharacterSimpleProjectile.MainCharacterSimpleProjectile_C" (`KismetMathLibrary.MakeTransform` (`self.K2_GetActorLocation`) (`self.K2_GetActorRotation`)) "Undefined" "OverrideRootScale" null (`self.ProjectileSpeed`) null)
        (goto _label_4)))))

(event `EnterPortal`
  (bind _returnvalue (`GameplayStatics.GetGameMode`))
  (bind _returnvalue_2 (`GameplayStatics.GetGameMode`))
  (if (`self.characterInPortal_Left`)
    (`PlayerCameraManager.StartCameraFade` (`GameplayStatics.GetPlayerCameraManager` 0) 0.0 1.0 0.5 (struct :`A` 1.0) false true)
    (`self.DisableInput` null)
    (set `CharacterMovementComponent.GravityScale` 0.0 (`self.CharacterMovement`))
    (bind _returnvalue_3 (`GameplayStatics.GetActorOfClass` "/Game/Presets/Portals.Portals_C"))
    (`/Game/Presets/Portals.HidePortals` _returnvalue_3)
    (`KismetSystemLibrary.Delay` 0.6)
    (`self.K2_SetActorRelativeLocation` (-810.0 0.0 110.0))
    (`|ExecutionSequence`
      (:`then_0`
        (bind _returnvalue_4 (`GameplayStatics.GetActorOfClass` "/Game/Presets/DungeonEntry.DungeonEntry_C"))
        (`/Engine/EditorBlueprintResources/StandardMacros.IsValid` _returnvalue_4
          (:`Is Valid`
            (`self.K2_DestroyActor` _returnvalue_4))))
      (:`then_1`
        (bind _asmain_game_mode (cast `/Game/MainCharacter/MainGameMode` _returnvalue_2))
        (bind _preset_ref (`/Game/MainCharacter/MainGameMode.Preset_Ref` _asmain_game_mode))
        (`/Engine/EditorBlueprintResources/StandardMacros.IsValid` _preset_ref
          (:`Is Valid`
            (`self.K2_DestroyActor` _preset_ref))))
      (:`then_2`
        (bind _asmain_game_mode_2 (cast `/Game/MainCharacter/MainGameMode` _returnvalue_2))
        (`/Game/MainCharacter/MainGameMode.RandomPresetLeftPortal` _asmain_game_mode_2)
        (`KismetSystemLibrary.Delay` 1.0)
        (set `CharacterMovementComponent.GravityScale` 1.0 (`self.CharacterMovement`))
        (`self.EnableInput` null)
        (`PlayerCameraManager.StartCameraFade` (`GameplayStatics.GetPlayerCameraManager` 0) 1.0 0.0 0.5 (struct :`A` 1.0) false false))
      (:`then_3`
        (bind _returnvalue_5 (`GameplayStatics.GetActorOfClass` "/Game/Presets/Portals.Portals_C"))
        (`/Game/Presets/Portals.UnhidePortalsAfterKillingMonsters` _returnvalue_5)))
    (elif (`self.characterInPortal_Right`)
      (`PlayerCameraManager.StartCameraFade` (`GameplayStatics.GetPlayerCameraManager` 0) 0.0 1.0 0.5 (struct :`A` 1.0) false true)
      (`self.DisableInput` null)
      (set `CharacterMovementComponent.GravityScale` 0.0 (`self.CharacterMovement`))
      (bind _returnvalue_6 (`GameplayStatics.GetActorOfClass` "/Game/Presets/Portals.Portals_C"))
      (`/Game/Presets/Portals.HidePortals` _returnvalue_6)
      (`KismetSystemLibrary.Delay` 0.6)
      (`self.K2_SetActorRelativeLocation` (-810.0 0.0 110.0))
      (`|ExecutionSequence`
        (:`then_0`
          (bind _returnvalue_7 (`GameplayStatics.GetActorOfClass` "/Game/Presets/DungeonEntry.DungeonEntry_C"))
          (`/Engine/EditorBlueprintResources/StandardMacros.IsValid` _returnvalue_7
            (:`Is Valid`
              (`self.K2_DestroyActor` _returnvalue_7))))
        (:`then_1`
          (bind _asmain_game_mode_3 (cast `/Game/MainCharacter/MainGameMode` _returnvalue))
          (bind _preset_ref_2 (`/Game/MainCharacter/MainGameMode.Preset_Ref` _asmain_game_mode_3))
          (`/Engine/EditorBlueprintResources/StandardMacros.IsValid` _preset_ref_2
            (:`Is Valid`
              (`self.K2_DestroyActor` _preset_ref_2))))
        (:`then_2`
          (bind _asmain_game_mode_4 (cast `/Game/MainCharacter/MainGameMode` _returnvalue))
          (`/Game/MainCharacter/MainGameMode.RandomPresetRightPortal` _asmain_game_mode_4)
          (`KismetSystemLibrary.Delay` 1.0)
          (set `CharacterMovementComponent.GravityScale` 1.0 (`self.CharacterMovement`))
          (`self.EnableInput` null)
          (`PlayerCameraManager.StartCameraFade` (`GameplayStatics.GetPlayerCameraManager` 0) 1.0 0.0 0.5 (struct :`A` 1.0) false false))
        (:`then_3`
          (bind _returnvalue_8 (`GameplayStatics.GetActorOfClass` "/Game/Presets/Portals.Portals_C"))
          (`/Game/Presets/Portals.UnhidePortalsAfterKillingMonsters` _returnvalue_8))))))

(event `Reload`
  ;[1 1 1] Fire Projectile
  (set `self.Reloading` true)
  (set `self.HoldFire` false)
  (`KismetSystemLibrary.Delay` (`self.FireRate`))
  (set `self.Reloading` false)
  (set `self.StartingBullet` true)
  (goto _label_5))

(event `self.CapsuleComponent.OnComponentBeginOverlap`
  (params (OverlappedComponent :type "PrimitiveComponent Object Reference") (OtherActor :type "Actor Object Reference") (OtherComp :type "PrimitiveComponent Object Reference") (OtherBodyIndex :type Integer) (bFromSweep :type Boolean) (SweepResult :type "HitResult Structure (by ref)"))
  ;[1 1 1] Getting Hit And Death
  (if (and (`ActorComponent.ComponentHasTag` OtherComp "Enemy") (not (`self.TemporaryImmortality`)))
    (set `self.LoseHP` true)
    (`self.DecrementCharacterHealth`)
    (elif (and (`ActorComponent.ComponentHasTag` OtherComp "EnemyProjectile") (not (`self.TemporaryImmortality`)))
      (`self.GetHitByProjectile`))))

(event `GetHitByProjectile`
  (bind _health (`self.Health`))
  ;[1 1 1] Getting Hit And Death
  (set `self.TemporaryImmortality` true)
  (set `self.Health` (`KismetMathLibrary.Clamp` (- _health 1) 0 _health))
  (`/Game/MainCharacter/Hud/WD_HUD.Decrease/IncreaseHealthOnHUD` (`self.WD_HUD_ref`))
  (if (== _health 0)
    (`self.PlayerDead`)
    (else
      (`KismetSystemLibrary.PrintString` (`KismetStringLibrary.Conv_IntToString` (`self.Health`)))
      (`KismetSystemLibrary.Delay` (`self.ImmortalityTime`))
      (set `self.TemporaryImmortality` false))))

(event `self.CapsuleComponent.OnComponentEndOverlap`
  (params (OverlappedComponent :type "PrimitiveComponent Object Reference") (OtherActor :type "Actor Object Reference") (OtherComp :type "PrimitiveComponent Object Reference") (OtherBodyIndex :type Integer))
  ;[1 1 1] Getting Hit And Death
  (if (`ActorComponent.ComponentHasTag` OtherComp "Enemy")
    (set `self.LoseHP` false)))

(event `DecrementCharacterHealth`
  (bind _health (`self.Health`))
  ;[1 1 1] Getting Hit And Death
  (if (and (`self.LoseHP`) (not (`self.TemporaryImmortality`)))
    (set `self.TemporaryImmortality` true)
    (set `self.Health` (`KismetMathLibrary.Clamp` (- _health 1) 0 _health))
    (`/Game/MainCharacter/Hud/WD_HUD.Decrease/IncreaseHealthOnHUD` (`self.WD_HUD_ref`))
    (if (== _health 0)
      (`self.PlayerDead`)
      (else
        (`KismetSystemLibrary.PrintString` (`KismetStringLibrary.Conv_IntToString` (`self.Health`)))
        (`KismetSystemLibrary.Delay` (`self.ImmortalityTime`))
        (set `self.TemporaryImmortality` false)
        (`self.DecrementCharacterHealth`)))))

(event `PlayerDead`
  ;[1 1 1] Getting Hit And Death
  (set `self.isPlayerDead?` true)
  (`self.DisableInput` (`GameplayStatics.GetPlayerController` 0))
  (`PlayerCameraManager.StartCameraFade` (`GameplayStatics.GetPlayerCameraManager` 0) 0.0 1.0 1.0 (struct :`A` 1.0) false true)
  (`KismetSystemLibrary.Delay` 1.5)
  (`GameplayStatics.OpenLevelBySoftObjectPtr` "/Game/HubLevel.HubLevel"))

(fn `CheckRightLeftOrientation`
  (returns (ReturnValue :type Boolean))
  (bind (_returnvalue_roll _returnvalue_pitch _returnvalue_yaw) (`KismetMathLibrary.BreakRotator` (`self.K2_GetActorRotation`)))
  (bind (_returnvalue_roll_2 _returnvalue_pitch_2 _returnvalue_yaw_2) (`KismetMathLibrary.BreakRotator` (`self.K2_GetActorRotation`)))
  (return (or (and (< _returnvalue_yaw -45.0) (> _returnvalue_yaw -135.0)) (and (> _returnvalue_yaw_2 45.0) (< _returnvalue_yaw_2 135.0)))))

(fn `CheckTopBotOrientation`
  (returns (ReturnValue :type Boolean))
  (bind (_returnvalue_roll _returnvalue_pitch _returnvalue_yaw) (`KismetMathLibrary.BreakRotator` (`self.K2_GetActorRotation`)))
  (bind (_returnvalue_roll_2 _returnvalue_pitch_2 _returnvalue_yaw_2) (`KismetMathLibrary.BreakRotator` (`self.K2_GetActorRotation`)))
  (return (or (and (>= _returnvalue_yaw -45.0) (<= _returnvalue_yaw 45.0)) (or (<= _returnvalue_yaw_2 -135.0) (>= _returnvalue_yaw_2 135.0)))))

(fn `UserConstructionScript`)