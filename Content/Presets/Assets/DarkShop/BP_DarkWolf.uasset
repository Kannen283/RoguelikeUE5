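; BP_DarkWolf is the merchant actor for the Dark Shop.
; On BeginPlay it spawns a BP_DarkWolf_Hat and snaps it onto the hat socket of the merchant's skeletal mesh.
; Its Box overlap events set InteractWithDarkShop on MainCharacter_BP when the player enters and clear it on exit, leaving the shop interaction itself outside this Blueprint.
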(event `self.ReceiveBeginPlay`
  (bind _returnvalue (`|SpawnActorFromClass` "/Game/Presets/Assets/DarkShop/BP_DarkWolf_Hat.BP_DarkWolf_Hat_C" (`SceneComponent.GetSocketTransform` (`self.MerchantSkeletalMesh`) "MerchantHat_Socket" "RTS_World") "Undefined" "OverrideRootScale" null null))
  (`self.K2_AttachToComponent` _returnvalue (`self.MerchantSkeletalMesh`) "MerchantHat_Socket" "SnapToTarget" "SnapToTarget" "SnapToTarget" true))

(event `self.Box.OnComponentBeginOverlap`
  (params (OverlappedComponent :type "PrimitiveComponent Object Reference") (OtherActor :type "Actor Object Reference") (OtherComp :type "PrimitiveComponent Object Reference") (OtherBodyIndex :type Integer) (bFromSweep :type Boolean) (SweepResult :type "HitResult Structure (by ref)"))
  (bind _asmain_character_bp (cast `/Game/MainCharacter/MainCharacter_BP` OtherActor))
  (set `/Game/MainCharacter/MainCharacter_BP.Interact_With_DarkShop?` true _asmain_character_bp))

(event `self.Box.OnComponentEndOverlap`
  (params (OverlappedComponent :type "PrimitiveComponent Object Reference") (OtherActor :type "Actor Object Reference") (OtherComp :type "PrimitiveComponent Object Reference") (OtherBodyIndex :type Integer))
  (bind _asmain_character_bp (cast `/Game/MainCharacter/MainCharacter_BP` OtherActor))
  (set `/Game/MainCharacter/MainCharacter_BP.Interact_With_DarkShop?` false _asmain_character_bp))

(fn `UserConstructionScript`)